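; Dragon character that roams and reacts to food on its own, and that the player can mount and control.
; A DragonState switch drives idle, sleep, eat and navmesh walking, with timers chaining single-node animations and picking random next states.
; Food overlap triggers eating unless asleep; overlapping the mount sphere while idle transfers player possession, and E restores both controllers.
; Flight logic is unfinished: the Fly state falls back to idle.
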(event OnComponentBeginOverlap(MountSphere)
  (params (OverlappedComponent :type Primitive%20Component%20Object%20Reference) (OtherActor :type Actor%20Object%20Reference) (OtherComp :type Primitive%20Component%20Object%20Reference) (OtherBodyIndex :type Integer) (bFromSweep :type Boolean) (SweepResult :type Hit%20Result%20Structure%20%28by%20ref%29))
  ;[1 1 1] Mount
  (if (and (== (Utilities|GetClass OtherActor) "/Game/Blueprints/BP_PlayerCharacter.BP_PlayerCharacter_C") (Utilities|Enum|Equal(Enum) (Variables|Default|GetDragonState) "NewEnumerator0"))
    (bind _output_get (Variables|Default|SetPlayerActor OtherActor))
    (Variables|Default|SetMyController (Pawn|GetController))
    (bind _asbp_player_character (Utilities|Casting|CastToBP_PlayerCharacter (Variables|Default|GetPlayerActor)))
    (if (Variables|/Game/Blueprints/BP_PlayerCharacter.BP_PlayerCharacter_C|GetisHoldingObject _asbp_player_character)
      (Default|DropObject _asbp_player_character))
    (Pawn|Possess (Game|GetPlayerController 0) self)
    (Collision|IgnoreActorwhenMoving (Variables|/Script/Engine.MovementComponent|GetUpdatedPrimitive (Variables|Character|GetCharacterMovement)) _output_get true)
    (Variables|Default|SetDragonState "NewEnumerator7")
    (CallFunction|HandleState)))

(event OnComponentBeginOverlap(FoodBox)
  (params (OverlappedComponent :type Primitive%20Component%20Object%20Reference) (OtherActor :type Actor%20Object%20Reference) (OtherComp :type Primitive%20Component%20Object%20Reference) (OtherBodyIndex :type Integer) (bFromSweep :type Boolean) (SweepResult :type Hit%20Result%20Structure%20%28by%20ref%29))
  (if (and (== (Utilities|GetClass OtherActor) "/Game/Blueprints/BP_Food.BP_Food_C") (Math|Boolean|NotEqual(Boolean) (Variables|Default|GetisSleeping) true))
    (Variables|Default|SetObjectToEat OtherActor)
    (Utilities|Time|ClearandInvalidateTimerbyHandle (Variables|Default|GetAnimTimerHandle))
    (Variables|Default|SetDragonState "NewEnumerator3")
    (CallFunction|HandleState)))

(event Custom|Play%20Idle
  (Utilities|Time|ClearandInvalidateTimerbyHandle (Variables|Default|GetAnimTimerHandle))
  (switch int (Math|Random|RandomIntegerinRange 0 2)
    (:0
      (Components|Animation|PlayAnimation (Variables|Character|GetMesh) "/Game/Dragon/Animations/Dragon_61_Anim_Idle.Dragon_61_Anim_Idle" false)
      (bind _returnvalue (Utilities|Time|SetTimerbyFunctionName 0 "State_SleepB,Walk,Fly" (* (Math|Random|RandomIntegerinRange 1 1) 22.15)))
      (Variables|Default|SetAnimTimerHandle _returnvalue))
    (:1
      (Components|Animation|PlayAnimation (Variables|Character|GetMesh) "/Game/Dragon/Animations/Dragon_61_Anim_Idle1.Dragon_61_Anim_Idle1" false)
      (bind _returnvalue_2 (Utilities|Time|SetTimerbyFunctionName 0 "State_SleepB,Walk,Fly" (* (Math|Random|RandomIntegerinRange 1 1) 10.7)))
      (Variables|Default|SetAnimTimerHandle _returnvalue_2))
    (:2
      (Components|Animation|PlayAnimation (Variables|Character|GetMesh) "/Game/Dragon/Animations/Dragon_61_Anim_Idle_Roar.Dragon_61_Anim_Idle_Roar" false)
      (bind _returnvalue_3 (Utilities|Time|SetTimerbyFunctionName 0 "State_SleepB,Walk,Fly" (* (Math|Random|RandomIntegerinRange 1 1) 11.0)))
      (Variables|Default|SetAnimTimerHandle _returnvalue_3))))

(event Custom|Play%20SleepBegin
  (Utilities|Time|ClearandInvalidateTimerbyHandle (Variables|Default|GetAnimTimerHandle))
  (Components|Animation|PlayAnimation (Variables|Character|GetMesh) "/Game/Dragon/Animations/Dragon_61_Anim_SleepStart_original.Dragon_61_Anim_SleepStart_original" false)
  (Variables|Default|SetisSleeping true)
  (bind _returnvalue (Utilities|Time|SetTimerbyFunctionName 0 "ChangeState_SleepL" 6.5))
  (Variables|Default|SetAnimTimerHandle _returnvalue))

(event Custom|Play_walk
  ;[1 1 1] Player Control
  (if (not (Variables|Default|Getctrl_IsWalking))
    (Components|Animation|PlayAnimation (Variables|Character|GetMesh) "/Game/Dragon/Animations/Dragon_61_Anim_Walk.Dragon_61_Anim_Walk" true)
    (Variables|Default|Setctrl_IsWalking true)
    (Variables|Default|Setctrl_isIdle false)))

(event Custom|State_SleepB,Walk,Fly
  (switch int (Math|Random|RandomIntegerinRange 0 2)
    (:Default
      _)
    (:0
      (Variables|Default|SetDragonState "NewEnumerator1"))
    (:1
      (Variables|Default|SetDragonState "NewEnumerator5"))
    (:2
      (Variables|Default|SetDragonState "NewEnumerator6")))
  (CallFunction|HandleState))

(event Custom|ChangeState_SleepB
  (Variables|Default|SetDragonState "NewEnumerator2")
  (CallFunction|HandleState))

(event Custom|Play_SleepLoop)

(event Custom|ChangeState_SleepL
  (Utilities|Time|ClearandInvalidateTimerbyHandle (Variables|Default|GetAnimTimerHandle))
  (bind _returnvalue (Utilities|Time|SetTimerbyFunctionName 0 "Play SleepEnd" 1.0))
  (Variables|Default|SetAnimTimerHandle _returnvalue))

(event Custom|ChangeState_SleepE)

(event Custom|ChangeState_EndOfSleep
  (Variables|Default|SetDragonState "NewEnumerator0")
  (Variables|Default|SetisSleeping false)
  (CallFunction|HandleState))

(event Custom|ChangeState_Eat_Start
  (Variables|Default|SetDragonState "NewEnumerator2")
  (CallFunction|HandleState))

(event Custom|HandleState
  (switch Utilities|FlowControl|Switch|SwitchonDragon_State (Variables|Default|GetDragonState)
    (:NewEnumerator0
      (CallFunction|PlayIdle :!label _label))
    (:NewEnumerator1
      (CallFunction|PlaySleepBegin))
    (:NewEnumerator2
      (CallFunction|PlaySleepEnd))
    (:NewEnumerator3
      (CallFunction|PlayEatStart (Variables|Default|GetObjectToEat)))
    (:NewEnumerator4
      (CallFunction|PlayEatEnd))
    (:NewEnumerator5
      (CallFunction|Walk))
    (:NewEnumerator6
      (goto _label))))

(event Custom|Play%20SleepEnd
  (Utilities|Time|ClearandInvalidateTimerbyHandle (Variables|Default|GetAnimTimerHandle))
  (Components|Animation|PlayAnimation (Variables|Character|GetMesh) "/Game/Dragon/Animations/Dragon_61_Anim_SleepStart_reverse.Dragon_61_Anim_SleepStart_reverse" true)
  (bind _returnvalue (Utilities|Time|SetTimerbyFunctionName 0 "ChangeState_EndOfSleep" 6.3))
  (Variables|Default|SetAnimTimerHandle _returnvalue))

(event Custom|Play%20Eat_Start
  (params (NewParam :type Actor%20Object%20Reference))
  (Utilities|Time|ClearandInvalidateTimerbyHandle (Variables|Default|GetAnimTimerHandle))
  (Components|Animation|PlayAnimation (Variables|Character|GetMesh) "/Game/Dragon/Animations/Dragon_61_Anim_Eat_Start.Dragon_61_Anim_Eat_Start" false)
  (bind _asbp_player_character (Utilities|Casting|CastToBP_PlayerCharacter (Game|Player|GetPlayerPawn 0)))
  (Default|ObjectHoldReset _asbp_player_character)
  (Actor|DestroyActor (Variables|Default|GetObjectToEat))
  (bind _returnvalue (Utilities|Time|SetTimerbyFunctionName 0 "ChangeState_Eat_Start" 4.0))
  (Variables|Default|SetAnimTimerHandle _returnvalue))

(event Custom|Play%20Eat_End
  ;[1 1 1] Not set up atm, since cannot create a duplicate of Bite_Begin (since UE4 crashes on save of a new duplicate)
  (Utilities|Time|ClearandInvalidateTimerbyHandle (Variables|Default|GetAnimTimerHandle))
  (Components|Animation|PlayAnimation (Variables|Character|GetMesh) "/Game/Dragon/Animations/Dragon_61_Anim_Eat_End.Dragon_61_Anim_Eat_End" false)
  (bind _returnvalue (Utilities|Time|SetTimerbyFunctionName 0 "State_SleepB,Walk,Fly" 4.0))
  (Variables|Default|SetAnimTimerHandle _returnvalue))

(event Custom|Walk
  (bind _capsulecomponent (Variables|Collision|GetCapsuleComponent))
  (bind _navdata (Variables|Default|GetNavData))
  (bind _returnvalue (Transformation|GetWorldLocation _capsulecomponent))
  (bind (_randomlocation _returnvalue_2) (Class|NavigationSystemV1|GetRandomPointinNavigableRadius _returnvalue 4e+03 _navdata 0))
  ;[1 1 1] Walking
  (Components|Animation|PlayAnimation (Variables|Character|GetMesh) "/Game/Dragon/Animations/Dragon_61_Anim_Walk.Dragon_61_Anim_Walk" true)
  (if _returnvalue_2
    (bind _movementresult (AI|AIMoveTo self _randomlocation 0 2e+01 false)
      (:OnSuccess
        (switch int (Math|Random|RandomIntegerinRange 0 1)
          (:Default
            (Variables|Default|SetDragonState "NewEnumerator0" :!label _label))
          (:0
            (Variables|Default|SetDragonState "NewEnumerator5"))))
      (:OnFail
        (Development|PrintString (Utilities|String|EnumtoString _movementresult))
        (goto _label)))
    (else
      (goto _label)))
  (CallFunction|HandleState))

(event Custom|Begin_Fly
  ;[1 1 1] Broken Flying
  (Components|Animation|PlayAnimation (Variables|Character|GetMesh) "/Game/Dragon/Animations/Dragon_61_Anim_Fly.Dragon_61_Anim_Fly" false) ; replace with some sort of begin fly
  (Variables|/Script/Engine.CharacterMovementComponent|SetGravityScale (Variables|Character|GetCharacterMovement) 0.0)
  (CallFunction|ContinueFly))

(event Custom|Continue_Fly
  (bind _flight_box (Variables|Default|GetFlight%20Box))
  (bind _collisioncomponent (Variables|/Script/Engine.TriggerBase|GetCollisionComponent _flight_box))
  ;[1 1 1] Broken Flying
  (Components|Animation|PlayAnimation (Variables|Character|GetMesh) "/Game/Dragon/Animations/Dragon_61_Anim_Fly.Dragon_61_Anim_Fly" true) ; Replace Fly With Gliding Anim
  (bind _asbox_collision (Utilities|Casting|CastToBoxComponent _collisioncomponent)
    (:then
      (bind _movementresult (AI|AIMoveTo self (Math|Random|RandomPointinBoundingBox (Transformation|GetWorldLocation _collisioncomponent) (Variables|/Script/Engine.BoxComponent|GetBoxExtent _asbox_collision)) 0 5.0 false)
        (:OnSuccess
          (switch int (Math|Random|RandomIntegerinRange 0 1)
            (:Default
              (CallFunction|EndFly :!label _label))
            (:0
              (CallFunction|ContinueFly))))
        (:OnFail
          (Development|PrintString (Utilities|String|EnumtoString _movementresult))
          (goto _label))))
    (:CastFailed
      (Development|PrintString "Flight Volume Not Box, Exiting"))))

(event Custom|End_Fly
  (bind _navdata (Variables|Default|GetNavData))
  (bind _middlelandinglocation (Variables|Default|GetMiddleLandingLocation))
  (bind (_randomlocation _returnvalue) (Class|NavigationSystemV1|GetRandomPointinNavigableRadius _middlelandinglocation 4e+03 _navdata 0))
  ;[1 1 1] Broken Flying
  (if _returnvalue
    (bind _movementresult (AI|AIMoveTo self _randomlocation 0 2e+01 false)
      (:OnSuccess
        (Variables|/Script/Engine.CharacterMovementComponent|SetGravityScale (Variables|Character|GetCharacterMovement) 1.0)
        (Components|Animation|PlayAnimation (Variables|Character|GetMesh) "/Game/Dragon/Animations/Dragon_61_Anim_Fly.Dragon_61_Anim_Fly" false) ; Replace With Landing Animation
        (Variables|Default|SetDragonState "NewEnumerator0")
        (CallFunction|HandleState))
      (:OnFail
        (Development|PrintString (Utilities|String|Append "Land Failed:" (Utilities|String|EnumtoString _movementresult)))
        (CallFunction|ContinueFly :!label _label)))
    (else
      (Development|PrintString "FlyStopFailed: Could not find point")
      (goto _label))))

(event EventBeginPlay
  (Variables|Default|SetDragonState (Variables|Default|GetStartState))
  (CallFunction|HandleState))

(event Collision|EventActorBeginOverlap
  (params (OtherActor :type Actor%20Object%20Reference)))

(event Input|AxisEvents|InputAxisMoveForward
  (params (AxisValue :type Float%20%28single-precision%29))
  ;[1 1 1] Player Control
  (if (== AxisValue 0.0)
    (if (not (Variables|Default|Getctrl_isIdle))
      (Components|Animation|PlayAnimation (Variables|Character|GetMesh) "/Game/Dragon/Animations/Dragon_61_Anim_Idle.Dragon_61_Anim_Idle" true)
      (Variables|Default|Setctrl_isIdle true)
      (Variables|Default|Setctrl_IsWalking false))
    (else
      (Pawn|Input|AddMovementInput (Transformation|GetActorForwardVector) AxisValue false)
      (CallFunction|PlayWalk))))

(event Input|AxisEvents|InputAxisMoveRight
  (params (AxisValue :type Float%20%28single-precision%29))
  ;[1 1 1] Player Control
  (if (not (== AxisValue 0.0))
    (Pawn|Input|AddControllerYawInput (* AxisValue (Utilities|Time|GetWorldDeltaSeconds) 15.0))))

(event Input|MouseEvents|MouseX
  (params (AxisValue :type Float%20%28single-precision%29))
  (bind _camera (Variables|Default|GetCamera))
  (bind _relativerotation (Variables|/Script/Engine.SceneComponent|GetRelativeRotation _camera))
  ;[1 1 1] Mounted Camera
  (Transformation|SetRelativeRotation (Variables|Default|GetCamera) (Math|Rotator|MakeRotator (.roll _relativerotation) (.pitch _relativerotation) (+ AxisValue (.yaw _relativerotation))) false false))

(event Input|MouseEvents|MouseY
  (params (AxisValue :type Float%20%28single-precision%29))
  (bind _camera (Variables|Default|GetCamera))
  (bind _relativerotation (Variables|/Script/Engine.SceneComponent|GetRelativeRotation _camera))
  ;[1 1 1] Mounted Camera
  (Transformation|SetRelativeRotation (Variables|Default|GetCamera) (Math|Rotator|MakeRotator (.roll _relativerotation) (+ AxisValue (.pitch _relativerotation)) (.yaw _relativerotation)) false false))

(event Input|KeyboardEvents|E
  (params (Key :type Key%20Structure))
  (bind _returnvalue (Transformation|GetActorLocation))
  ;[1 1 1] Dismount
  (:Pressed
    (Transformation|SetActorLocation (Variables|Default|GetPlayerActor) (Math|Vector|MakeVector (.x _returnvalue) (- (.y _returnvalue) 5e+02) (- (.z _returnvalue) 3e+02)) false false)
    (bind _asbp_player_character (Utilities|Casting|CastToBP_PlayerCharacter (Variables|Default|GetPlayerActor)))
    (Pawn|Possess (Game|GetPlayerController 0) _asbp_player_character)
    (Pawn|Possess (Variables|Default|GetMyController) self)
    (Variables|Default|SetDragonState "NewEnumerator0")
    (CallFunction|HandleState)))

(event Input|KeyboardEvents|SpaceBar
  (params (Key :type Key%20Structure))
  (:Pressed
    (Development|PrintString "Hello")))

(event Input|KeyboardEvents|Y
  (params (Key :type Key%20Structure))
  ;[1 1 1] Fix Camera rotation when bugged
  (:Pressed
    (Transformation|SetWorldRotation (Variables|Default|GetCamera) (Transformation|GetWorldRotation (Variables|Collision|GetCapsuleComponent)) false false)))

(fn ConstructionScript)