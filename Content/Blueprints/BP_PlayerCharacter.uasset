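; First-person player character that picks up, drops and throws physics objects, clicks interactables and can teleport.
; Left click gaze-traces for BPI_Pickup or BPI_Clickable actors; a PhysicsHandle carries grabbed components, updated each Tick.
; Holding right click oscillates throw strength along a cosine until release.
; In teleport mode, Tick traces a segmented parabola to find floor-like surfaces for left-click teleporting, but the mode toggle and older straight-line teleport are disconnected.
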(event Custom|Object_Hold_Reset
  (if (Variables|Default|GetisHoldingObject)
    (Variables|Default|SetisHoldingObject false)))

(event Custom|DropObject
  ;[1 1 1] Drop Object in Hand
  (if (Variables|Default|GetisHoldingObject)
    (Physics|Components|PhysicsHandle|ReleaseComponent (Variables|Default|GetPhysicsHandle))
    (Variables|Default|SetisHoldingObject false)
    (Utilities|FlowControl|Delay 0.2)
    (Collision|SetCollisionResponsetoChannel (Variables|Default|GetHeldObject) "ECC_Pawn" "ECR_Block")))

(event Custom|GazeCheck
  (bind _firstpersoncameracomponent (Variables|Default|GetFirstPersonCameraComponent))
  (bind _returnvalue (Transformation|GetWorldLocation _firstpersoncameracomponent))
  ;[1 1 1] GazeCheck - Check if there is an object we can interact with in front of us (Implements either BPI_Pickup or BPI_Clickable)
  (bind (_outhit _returnvalue_2) (Collision|LineTraceByChannel _returnvalue (+ _returnvalue (* (Math|Vector|GetForwardVector _firstpersoncameracomponent) 3e+02)) "TraceTypeQuery1" false 0 "None"))
  (if _returnvalue_2
    (if (Utilities|DoesObjectImplementInterface (.HitActor (Collision|BreakHitResult _outhit)) "/Game/Blueprints/BPI_Pickup.BPI_Pickup_C")
      (Variables|Default|SetHeldActor (.HitActor (Collision|BreakHitResult _outhit)))
      (Utilities|IsValid (Variables|Default|GetHeldActor)
        (:Is%20Valid
          (Class|BPIPickup|PickUp(Message) (Variables|Default|GetHeldActor))
          (CallFunction|PickUpObject (.HitComponent (Collision|BreakHitResult _outhit)))))
      (elif (Utilities|DoesObjectImplementInterface (.HitActor (Collision|BreakHitResult _outhit)) "/Game/Blueprints/BPI_Clickable.BPI_Clickable_C")
        (Utilities|IsValid (.HitActor (Collision|BreakHitResult _outhit))
          (:Is%20Valid
            (Class|BPIClickable|ClickonObject(Message) (.HitActor (Collision|BreakHitResult _outhit)))))))))

(event Custom|PickUpObject
  (params (NewParam :type Primitive%20Component%20Object%20Reference))
  ;[1 1 1] PickUp Object (if object simulates Physics)
  (if (Physics|IsSimulatingPhysics NewParam "None")
    (bind _output_get (Variables|Default|SetHeldObject NewParam))
    (Transformation|SetWorldRotation (Variables|Default|GetHeldObjectLocation) (.rotation (Transformation|GetWorldTransform _output_get)) false false)
    (Physics|Components|PhysicsHandle|GrabComponentatLocationwithRotation (Variables|Default|GetPhysicsHandle) (Variables|Default|GetHeldObject) "None" (.location (Transformation|GetWorldTransform _output_get)) (.rotation (Transformation|GetWorldTransform _output_get)))
    (Collision|SetCollisionResponsetoChannel (Variables|Default|GetHeldObject) "ECC_Pawn" "ECR_Ignore")
    (Variables|Default|SetisHoldingObject true)
    (else
      (Development|PrintString "Target Implements BPI_Pickup but does not simulate physics."))))

(event Custom|DrawTeleportCurve
  (bind _firstpersoncameracomponent (Variables|Default|GetFirstPersonCameraComponent))
  ;[1 1 1] Draw Teleport Curve if TeleportMode Enabled
  (if (Variables|Default|GetbModeTeleport)
    (CallFunction|GetTeleportLocationParabola (Transformation|GetWorldLocation _firstpersoncameracomponent) (Math|Vector|GetForwardVector _firstpersoncameracomponent) 50 0.1 (Variables|Default|GetTestSpeed))))

(event Custom|UpdateHeldItemTransform
  (bind _heldobjectlocation (Variables|Default|GetHeldObjectLocation))
  ;[1 1 1] Update location and rotation of held item
  (Class|PhysicsHandleComponent|SetTargetLocationandRotation (Variables|Default|GetPhysicsHandle) (Transformation|GetWorldLocation _heldobjectlocation) (Transformation|GetWorldRotation _heldobjectlocation)))

(event Custom|ThrowObject
  ;[1 1 1] Throw
  (if (Variables|Default|GetisHoldingObject)
    (Physics|Components|PhysicsHandle|ReleaseComponent (Variables|Default|GetPhysicsHandle))
    (Variables|Default|SetisHoldingObject false)
    (Collision|SetCollisionResponsetoChannel (Variables|Default|GetHeldObject) "ECC_Pawn" "ECR_Block")
    (Class|PrimitiveComponent|SetAllPhysicsLinearVelocity (Variables|Default|GetHeldObject) (* (Math|Vector|GetForwardVector (Variables|Default|GetFirstPersonCameraComponent)) (* (Variables|Default|GetThrowForcePercent) (Variables|Default|GetThrowForce))) false)))

(event Custom|CalculateThrowForce
  ;[1 1 1] Calculates Throw Force if holding down button
  (if (Variables|Default|GetisHoldingObject)
    (if (Variables|Default|GetThrowWindUp)
      (bind _output_get (Variables|Default|SetThrowHelper (+ (Variables|Default|GetThrowHelper) (* (Variables|Default|GetDeltaTime) (Variables|Default|GetThrowCycleSpeed)))))
      (Variables|Default|SetThrowForcePercent (- 1.0 (Math|Float|Absolute(Float) (Math|Trig|Cos(Radians) _output_get)))))))

(event EventBeginPlay
  (bind _returnvalue (UserInterface|CreateWidget "/Game/Blueprints/WBP_PlayerUI.WBP_PlayerUI_C" (Game|GetPlayerController 0)))
  (UserInterface|Viewport|AddtoViewport _returnvalue 0))

(event Collision|EventActorBeginOverlap
  (params (OtherActor :type Actor%20Object%20Reference)))

(event EventTick
  (params (DeltaSeconds :type Float%20%28single-precision%29))
  (Variables|Default|SetDeltaTime DeltaSeconds)
  (CallFunction|UpdateHeldItemTransform)
  (CallFunction|DrawTeleportCurve)
  (CallFunction|CalculateThrowForce))

(event Input|MouseEvents|RightMouseButton
  (params (Key :type Key%20Structure))
  ;[1 1 1] Input (Right Click) - Throw items
  (:Pressed
    (Variables|Default|SetThrowHelper 0.0)
    (Variables|Default|SetThrowWindUp true))
  (:Released
    (Variables|Default|SetThrowWindUp false)
    (CallFunction|ThrowObject)
    (Variables|Default|SetThrowForcePercent 0.0)))

(event Input|MouseEvents|RightMouseButton
  (params (Key :type Key%20Structure))
  ;[1 1 1] Old Teleport (straight line)
)

(event Input|KeyboardEvents|E
  (params (Key :type Key%20Structure))
  ;[1 1 1] Press E to Toggle Point and Click Teleport
)

(event Input|MouseEvents|LeftMouseButton
  (params (Key :type Key%20Structure))
  ;[1 1 1] Input (Left Click) - Pickup/Drop items and Teleport to Location
  (:Pressed
    (if (Variables|Default|GetbModeTeleport)
      (if (Variables|Default|GetbCanTeleport)
        (CallFunction|TeleporttoLocation (Variables|Default|GetTeleportLocation))
        (Development|PrintString "Teleport Location Acceptable"))
      (elif (Variables|Default|GetisHoldingObject)
        (CallFunction|DropObject)
        (else
          (CallFunction|GazeCheck))))))

(fn ConstructionScript)

(fn ToggleModeTeleport
  (if (Variables|Default|GetbModeTeleport)
    (Development|PrintString "ModeTeleport: OFF")
    (Variables|Default|SetbModeTeleport false)
    (else
      (Development|PrintString "ModeTeleport: ON")
      (Variables|Default|SetbModeTeleport true))))

(fn GetTeleportLocationParabola
  (params (Location :type Vector) (Forward :type Vector) (Steps :type Integer) (TimeStep :type Float%20%28single-precision%29) (Speed :type Float%20%28single-precision%29))
  (Utilities|FlowControl|Sequence
    (:then_0
      (bind _output_get (LocalVariables|SetInitialLocation Location))
      (LocalVariables|SetPreviousLocation _output_get)
      (LocalVariables|SetVelocity (* Forward Speed))
      (LocalVariables|SetTime TimeStep))
    (:then_1
      (bind _index (Utilities|FlowControl|ForLoopwithBreak 1 Steps :!label _label)
        (:LoopBody
          ;[1 1 1] missing interactive, teleport
          (bind (_outhit _returnvalue) (Collision|LineTraceByChannel (LocalVariables|GetPreviousLocation) (+ (Math|Vector|MakeVector (* (.X (Math|Vector|BreakVector (LocalVariables|GetVelocity))) (* _index (LocalVariables|GetTime))) (* (.Y (Math|Vector|BreakVector (LocalVariables|GetVelocity))) (* _index (LocalVariables|GetTime))) (- (* (.Z (Math|Vector|BreakVector (LocalVariables|GetVelocity))) (* _index (LocalVariables|GetTime))) (* (* _index (LocalVariables|GetTime)) (* _index (LocalVariables|GetTime)) 0.5 (Variables|Default|GetTestGravity)))) (LocalVariables|GetInitialLocation)) "TraceTypeQuery3" false 0 "ForOneFrame" true "(R=1.000000,G=0.009645,B=0.000000,A=1.000000)"))
          (LocalVariables|SetPreviousLocation (+ (Math|Vector|MakeVector (* (.X (Math|Vector|BreakVector (LocalVariables|GetVelocity))) (* _index (LocalVariables|GetTime))) (* (.Y (Math|Vector|BreakVector (LocalVariables|GetVelocity))) (* _index (LocalVariables|GetTime))) (- (* (.Z (Math|Vector|BreakVector (LocalVariables|GetVelocity))) (* _index (LocalVariables|GetTime))) (* (* _index (LocalVariables|GetTime)) (* _index (LocalVariables|GetTime)) 0.5 (Variables|Default|GetTestGravity)))) (LocalVariables|GetInitialLocation)))
          (if _returnvalue
            (Utilities|FlowControl|Sequence
              (:then_0
                (goto _label Break))
              (:then_1
                (if (> (Math|Vector|DotProduct (.Normal (Collision|BreakHitResult _outhit)) "0, 0,1.000000") 0.5)
                  (bind _output_get_2 (Variables|Default|SetbCanTeleport (> (Math|Vector|DotProduct (.Normal (Collision|BreakHitResult _outhit)) "0, 0,1.000000") 0.5)))
                  (if _output_get_2
                    (bind _output_get_3 (Variables|Default|SetTeleportLocation (.Location (Collision|BreakHitResult _outhit))))
                    (Class|KismetSystemLibrary|DrawDebugCylinder _output_get_3 (+ _output_get_3 (* (.Normal (Collision|BreakHitResult _outhit)) 1e+01)) 3e+01 25 "(R=0.000000,G=0.542093,B=1.000000,A=1.000000)" 0.0 1.0)))))
            (else
              (Variables|Default|SetbCanTeleport false))))))))

(fn TeleporttoLocation
  (params (Location :type Vector))
  (Transformation|SetActorLocation (Math|Vector|MakeVector (.x Location) (.y Location) (+ (.z Location) (Variables|/Script/Engine.CapsuleComponent|GetCapsuleHalfHeight (Variables|Default|GetCapsuleComponent)))) false false))